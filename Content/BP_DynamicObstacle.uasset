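; BP_DynamicObstacle is an obstacle whose cube starts moving and spinning randomly when play begins.
; BeginPlay rolls two random floats from a range based on RandBound, then applies them to the Cube as a one-time linear impulse on X and Z.
; The same two values, swapped onto X and Y, drive an angular impulse, so drift and spin are linked and physics carries the motion afterward.
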(event `self.ReceiveBeginPlay`
  (`self.Set Rands`)
  (`self.Start Impulse`)
  (`self.Start Rotation`))

(fn `Get Rand`
  (returns (`New Rand` :type "Float (double-precision)"))
  (bind _randbound (`self.RandBound`))
  (bind _result (`/Engine/EditorBlueprintResources/StandardMacros.NegateFloat` _randbound)
    (:`  `
      (return (`KismetMathLibrary.RandomFloatInRange` _result _randbound)))))

(fn `Set Rands`
  (bind _new_rand (`self.Get Rand` self))
  (set `self.Rand1` _new_rand)
  (bind _new_rand_2 (`self.Get Rand` self))
  (set `self.Rand2` _new_rand_2))

(fn `Start Impulse`
  (`PrimitiveComponent.AddImpulse` (`self.Cube`) (`KismetMathLibrary.MakeVector` (`self.Rand1`) 0.0 (`self.Rand2`)) "None" false))

(fn `Start Rotation`
  (`PrimitiveComponent.AddAngularImpulse` (`self.Cube`) (`KismetMathLibrary.MakeVector` (`self.Rand2`) (`self.Rand1`)) "None" false))

(fn `UserConstructionScript`
  (`parent.UserConstructionScript`))