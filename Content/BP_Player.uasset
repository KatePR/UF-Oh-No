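; Player Blueprint that takes over the view with its own camera and manages a fuel supply shown through an on-screen fuel bar.
; Fuel starts full; SubtractFuel drains it and runs CheckWarnings, which toggles a low-fuel warning widget below a quarter tank and calls LoseGame on the game mode when empty.
; AddFuel always refills to maximum because its branch condition is hardwired true, leaving the additive path unused.
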(event `self.ReceiveBeginPlay`
  (`self.Set Camera`)
  (`self.Set Starting Fuel`)
  (`self.Show Fuel Bar`))

(fn `Add Fuel`
  (params (Fuel_Value :type "Float (double-precision)"))
  (if true
    (set `self.Current_Fuel` (`self.Max_Fuel`))
    (else
      (set `self.Current_Fuel` (+ (`self.Current_Fuel`) (`local.Fuel_Value`))))))

(fn `Check Warnings`
  (bind _newparam (`self.Get Fuel Percentage`))
  (if (`KismetMathLibrary.InRange_FloatFloat` _newparam 0.0 0.25 false)
    (if (not (`self.Warning Is On`))
      (set `self.Warning Is On` true)
      (`self.Set Warning` true))
    (else
      (set `self.Warning Is On` false)
      (`self.Set Warning` false)
      (if (<= (`self.Current_Fuel`) 0.0)
        (bind _asmy_game_mode (cast `/Game/My_Game_Mode` (`GameplayStatics.GetGameMode`)))
        (`/Game/My_Game_Mode.Lose_Game` _asmy_game_mode)))))

(fn `Get Fuel Percentage`
  (returns (NewParam :type "Float (double-precision)"))
  (return (/ (`self.Current_Fuel`) (`self.Max_Fuel`))))

(fn `HasFuel`
  (returns (NewParam :type Boolean))
  (return (> (`self.Current_Fuel`) 0.0)))

(fn `Set Camera`
  (`ActorComponent.Activate` (`self.Main_Camera`) false)
  (`PlayerController.SetViewTargetWithBlend` (`GameplayStatics.GetPlayerController` 0) self 0.0 "VTBlend_Linear" 0.0 false))

(fn `Set Starting Fuel`
  (set `self.Current_Fuel` (`self.Max_Fuel`)))

(fn `Set Warning`
  (params (`Turn On/Off` :type Boolean))
  (if `Turn On/Off`
    (bind _returnvalue (`|CreateWidget` "/Game/Fuel_Warning.Fuel_Warning_C" (`GameplayStatics.GetPlayerController` 0)))
    (`UserWidget.AddToViewport` _returnvalue 0)
    (else
      (bind _foundwidgets (`WidgetBlueprintLibrary.GetAllWidgetsOfClass` "/Game/Fuel_Warning.Fuel_Warning_C"))
      (for _array_element _foundwidgets
        (`Widget.RemoveFromParent` _array_element)))))

(fn `Show Fuel Bar`
  (bind _returnvalue (`|CreateWidget` "/Game/Fuel_Bar.Fuel_Bar_C" (`GameplayStatics.GetPlayerController` 0)))
  (`UserWidget.AddToViewport` _returnvalue 0))

(fn `Subtract Fuel`
  (params (Fuel :type "Float (double-precision)"))
  (set `self.Current_Fuel` (- (`self.Current_Fuel`) Fuel))
  (`self.Check Warnings`))

(fn `UserConstructionScript`)